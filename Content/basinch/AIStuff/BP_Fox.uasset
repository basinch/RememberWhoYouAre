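; Fox AI character that hunts the player, or flees while the player's Dino flag is set.
; A self-restarting AI MoveTo loop runs while alive, playing an attack montage when it arrives within range.
; PerformAttack, not called here, damages the player on any sphere-trace hit, while Damage kills the fox and destroys it after a short delay.
; Egg-projectile, mouse-aim and several other helper functions go uncalled in this graph.
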(event `self.ReceiveBeginPlay`
  (bind _asbp_third_person_character (cast `/Game/ThirdPerson/Blueprints/BP_ThirdPersonCharacter` (`GameplayStatics.GetPlayerCharacter` 0)))
  (set `self.As BP Third Person Character` _asbp_third_person_character)
  (`self.StartMoving`))

(event `StartMoving`
  (bind _as_bp_third_person_character (`self.As BP Third Person Character`))
  (bind _dino (`/Game/ThirdPerson/Blueprints/BP_ThirdPersonCharacter.Dino` _as_bp_third_person_character))
  (if _dino :!label _label
    (`|AIMoveTo` self (`self.GetFarPoint` 300.0) null
      (:`OnSuccess`
        _)
      (:`OnFail`
        _))
    (else
      (`|AIMoveTo` self (0.0 0.0 0.0) _as_bp_third_person_character
        (:`OnSuccess`
          (if _dino
            _
            (elif (`self.GetDistance` 200.0)
              (`|PlayMontage` (`self.Mesh`) "/Game/basinch/Assets/fox/fox_AttackMontage.fox_AttackMontage"
                (:`OnCompleted`
                  _)
                (:`OnBlendOut`
                  _)
                (:`OnInterrupted`
                  _)))))
        (:`OnFail`
          _))))
  (if (`self.Alive`)
    (goto _label)))

(event `/Game/basinch/BPI_Attack.PerformAttack`
  (bind _returnvalue (`SceneComponent.GetSocketLocation` (`self.Mesh`) "spine_009"))
  (bind (_outhit _returnvalue_2) (`KismetSystemLibrary.SphereTraceSingle` :`Start` _returnvalue :`End` (+ (* (`SceneComponent.GetForwardVector` (`self.Mesh`)) -50) _returnvalue) :`Radius` 50.0 :`TraceChannel` "TraceTypeQuery1" :`DrawDebugType` "ForDuration" :`DrawTime` 1.0))
  (if _returnvalue_2
    (`GameplayStatics.ApplyDamage` (`self.As BP Third Person Character`) 1.0)))

(event `Die`
  (bind _mesh (`self.Mesh`))
  (bind _capsulecomponent (`self.CapsuleComponent`))
  (set `self.Alive` false)
  (`PrimitiveComponent.SetCollisionProfileName` (`self.Mesh`) "Blockall" true)
  (`SceneComponent.K2_SetWorldRotation` _mesh (struct :`Roll` 90.0) false false)
  (`SceneComponent.K2_SetWorldRotation` _capsulecomponent (struct :`Roll` 90.0) false false)
  (`PrimitiveComponent.SetCollisionProfileName` _capsulecomponent "NoCollision" true)
  (`PrimitiveComponent.SetCollisionEnabled` _mesh "NoCollision")
  (`SkeletalMeshComponent.SetAnimInstanceClass` _mesh null)
  (`KismetSystemLibrary.Delay` 0.4)
  (`self.K2_DestroyActor`))

(event `/Game/basinch/BPI_Damage.Damage`
  (`self.Die`))

(fn `CanEnterShtngMde`
  (returns (ReturnValue :type Boolean))
  (return (not (`self.IsJumping`))))

(fn `GetDistance`
  (params (MinDistance :type "Float (double-precision)"))
  (returns (ReturnValue :type Boolean) (ReturnValue1 :type "Float (double-precision)"))
  (bind _returnvalue (`KismetMathLibrary.Vector_Distance` (`self.K2_GetActorLocation`) (`self.K2_GetActorLocation` (`self.As BP Third Person Character`))))
  (return (<= _returnvalue MinDistance) _returnvalue))

(fn `GetFarPoint`
  (params (MinDistance :type "Float (double-precision)"))
  (returns (Output_Get :type "Vector Structure"))
  (return (+ (* (* MinDistance -1.0) (`KismetMathLibrary.Normal` (- (`self.K2_GetActorLocation` (`self.As BP Third Person Character`)) (`self.K2_GetActorLocation`)))) (`self.K2_GetActorLocation`))))

(fn `GetNearPoint`
  (params (MinDistance :type "Float (double-precision)"))
  (returns (Output_Get :type "Vector Structure"))
  (return (+ (* (`KismetMathLibrary.Normal` (- (`self.K2_GetActorLocation` (`self.As BP Third Person Character`)) (`self.K2_GetActorLocation`))) MinDistance) (`self.K2_GetActorLocation`))))

(fn `IsJumping`
  (returns (ReturnValue :type Boolean))
  (return (`NavMovementInterface.IsFalling` (`self.CharacterMovement`))))

(fn `LookAtMouse`
  (params (Target :type "Vector Structure (by ref)"))
  (bind (_returnvalue_roll _returnvalue_pitch) (`KismetMathLibrary.BreakRotator` (`self.K2_GetActorRotation`)))
  (`self.K2_SetActorRotation` (`KismetMathLibrary.MakeRotator` _returnvalue_roll _returnvalue_pitch (.yaw (`KismetMathLibrary.FindLookAtRotation` (`self.K2_GetActorLocation`) Target)))))

(fn `MouseTraceWorldLocation`
  (returns (ReturnValue :type Boolean) (OutHit :type "HitResult Structure"))
  (bind (_worldlocation _worlddirection) (`PlayerController.DeprojectMousePositionToWorld` (`GameplayStatics.GetPlayerController` 0)))
  (bind (_outhit _returnvalue) (`KismetSystemLibrary.LineTraceSingle` _worldlocation (+ (* _worlddirection 5000) _worldlocation) "TraceTypeQuery1"))
  (return _returnvalue _outhit))

(fn `SpawnEggProjectile`
  (`|SpawnActorFromClass` "/Game/basinch/BP_EggProjectile.BP_EggProjectile_C" (`KismetMathLibrary.MakeTransform` (`SceneComponent.K2_GetComponentLocation` (`self.Scene`)) (`KismetMathLibrary.MakeRotator` (.roll (`self.K2_GetActorRotation`)) (.pitch (`self.K2_GetActorRotation`)) (+ (.yaw (`self.K2_GetActorRotation`)) 180.0))) "AlwaysSpawn" "MultiplyWithRoot" null 1500.0 null))

(fn `TraceLocations`
  (params (Radius :type "Float (double-precision)"))
  (returns (StartLocation :type "Vector Structure") (EndLocation :type "Vector Structure"))
  (bind _returnvalue (+ (* (`SceneComponent.GetForwardVector` (`self.CapsuleComponent`)) Radius) (`SceneComponent.GetSocketLocation` (`self.Mesh`) "head")))
  (return _returnvalue (`KismetMathLibrary.MakeVector` (.x _returnvalue) (.y _returnvalue) (- (.z _returnvalue) 150.0))))

(fn `UserConstructionScript`)