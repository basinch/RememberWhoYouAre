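; Enemy spawner actor that spawns a requested number of BP_Fox enemies in a line, one at a time.
; Spawnenemy stores the count and starts a looping timer at Spawndelay intervals that fires Spawntilki.
; Each tick places a fox at an evenly growing offset along the enum-selected X or Y axis, facing the player.
; The timer clears once SpawnedAmount reaches the count; the counter is never reset here.
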(event `Spawnenemy`
  (params (Spawncount :type Integer))
  (set `self.Spawncount` Spawncount)
  (bind _returnvalue (`KismetSystemLibrary.K2_SetTimerDelegate` (delegate `Spawntilki`) (`self.Spawndelay`) true))
  (set `self.Spawn` _returnvalue))

(event `Spawntilki`
  (bind _returnvalue (+ (`self.K2_GetActorLocation`) (select `/Game/basinch/E_Yon` (`self.enum`) :`NewEnumerator0` (`KismetMathLibrary.MakeVector` (`KismetMathLibrary.Conv_IntToDouble` (* (`self.SpawnedAmount`) 150)) 0.0 40.0) :`NewEnumerator1` (`KismetMathLibrary.MakeVector` 0.0 (`KismetMathLibrary.Conv_IntToDouble` (* (`self.SpawnedAmount`) 150)) 40.0))))
  (`|SpawnActorFromClass` "/Game/basinch/AIStuff/BP_Fox.BP_Fox_C" (`KismetMathLibrary.MakeTransform` _returnvalue (`KismetMathLibrary.FindLookAtRotation` _returnvalue (`self.K2_GetActorLocation` (`GameplayStatics.GetPlayerCharacter` 0)))) "AlwaysSpawn" "MultiplyWithRoot" null null)
  (`/Engine/EditorBlueprintResources/StandardMacros.IncrementInt` (`self.SpawnedAmount`)
    (:`  `
      (if (>= (`self.SpawnedAmount`) (`self.Spawncount`))
        (`KismetSystemLibrary.K2_ClearAndInvalidateTimerHandle` (`self.Spawn`))))))

(fn `UserConstructionScript`)