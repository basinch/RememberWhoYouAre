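; BP_ChickCamera is a standalone follow camera actor that becomes the first player's view target on BeginPlay.
; Each tick it teleports toward the player character's capsule location, smoothed with VInterpTo at a configurable InterpSpeed.
; The construction script sets the spring arm length from the Height variable, which controls the camera's distance from the followed point.
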(event `self.ReceiveBeginPlay`
  (`PlayerController.SetViewTargetWithBlend` (`GameplayStatics.GetPlayerController` 0) (`ActorComponent.GetOwner` (`self.Camera`)) 0.0 "VTBlend_Linear" 0.0 false))

(event `self.ReceiveTick`
  (params (DeltaSeconds :type "Float (single-precision)"))
  (`self.K2_SetActorLocation` (`self.GetPlayerVinterpLocation` DeltaSeconds) false true))

(fn `GetPlayerVinterpLocation`
  (params (DeltaTime :type "Float (single-precision)"))
  (returns (ReturnValue :type "Vector Structure"))
  (bind (_returnvalue_x _returnvalue_y _returnvalue_z) (`KismetMathLibrary.BreakVector` (`SceneComponent.K2_GetComponentLocation` (`Character.CapsuleComponent` (`GameplayStatics.GetPlayerCharacter` 0)))))
  (return (`KismetMathLibrary.VInterpTo` (`SceneComponent.K2_GetComponentLocation` (`self.DefaultSceneRoot`)) (`KismetMathLibrary.MakeVector` _returnvalue_x _returnvalue_y _returnvalue_z) DeltaTime (`self.Interp Speed`))))

(fn `UserConstructionScript`
  (set `SpringArmComponent.TargetArmLength` (`self.Height`) (`self.SpringArm`)))