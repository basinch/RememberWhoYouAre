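; BP_FallTree is a tree actor that topples over when its Damage event is called.
; Damage plays a timeline from the start, using its float track as the alpha to lerp the Tree component's relative pitch toward 90 degrees while keeping roll and yaw.
; Each update lerps from the current rotation rather than a stored start, so the motion compounds instead of following the curve directly.
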(event `/Game/basinch/BPI_Damage.Damage`
  (bind _tree (`self.Tree`))
  (bind (_relativerotation_roll _relativerotation_pitch _relativerotation_yaw) (`KismetMathLibrary.BreakRotator` (`SceneComponent.RelativeRotation` _tree)))
  (bind (_direction _newtrack_0) (`Timeline|Timeline` :!via `PlayFromStart`)
    (:`Update`
      (`SceneComponent.K2_SetRelativeRotation` _tree (`KismetMathLibrary.RLerp` (`KismetMathLibrary.MakeRotator` _relativerotation_roll _relativerotation_pitch _relativerotation_yaw) (`KismetMathLibrary.MakeRotator` _relativerotation_roll 90.0 _relativerotation_yaw) _newtrack_0) false false))))

(fn `UserConstructionScript`
  (`parent.UserConstructionScript`))